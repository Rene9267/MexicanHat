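; BP_HatStair spawns a vertical stack of BP_HatStack actors at its own location.
; The HatStack event prints its input, then divides twice that value by an adjusted HatHeight, rounding up to set the loop's end index.
; Each spawn rises by a truncated HatOffset step.
; When the division leaves no positive remainder, only the first spawn gets a location; the rest use the default transform.
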(event Custom|Hat%20Stack
  (params (NewParam :type Float%20%28single-precision%29))
  (bind _returnvalue (Transformation|GetActorTransform))
  (bind _returnvalue_2 (Transformation|GetActorTransform))
  (bind _returnvalue_3 (* 2 NewParam))
  (bind _hat_height (Variables|Default|GetHat%20Height))
  (bind _returnvalue_4 (- _hat_height 3.5))
  (bind (_remainder _returnvalue_5) (Math|Float|Division(WholeandRemainder) _returnvalue_3 _returnvalue_4))
  (Development|PrintString (Utilities|String|ToString(Float) NewParam))
  (if (> _remainder 0.0)
    (bind _output_get (Variables|Default|SetNumber%20for%20top (+ _returnvalue_5 1)))
    (for _index (range 0 _output_get)
      (Game|SpawnActorfromClass "/Game/BluePrint/BP_HatStack.BP_HatStack_C" (Math|Transform|MakeTransform (Math|Vector|MakeVector (.x (.location _returnvalue)) (.y (.location _returnvalue)) (+ (.z (.location _returnvalue)) (Math|Conversions|ToFloat(Integer) (* _index (Math|Float|Truncate (Variables|Default|GetHat%20Offset)))))) "0, 0, 0" "1,1,1") "Undefined" 0 0))
    (else
      (bind _output_get_2 (Variables|Default|SetNumber%20for%20top _returnvalue_5))
      (for _index_2 (range 0 _output_get_2)
        (if (== _index_2 0)
          (Game|SpawnActorfromClass "/Game/BluePrint/BP_HatStack.BP_HatStack_C" (Math|Transform|MakeTransform (Math|Vector|MakeVector (.x (.location _returnvalue_2)) (.y (.location _returnvalue_2)) (+ (.z (.location _returnvalue_2)) (Math|Conversions|ToFloat(Integer) (* _index_2 (Math|Float|Truncate (Variables|Default|GetHat%20Offset)))))) "0, 0, 0" "1,1,1") "Undefined" 0 0)
          (else
            (Game|SpawnActorfromClass "/Game/BluePrint/BP_HatStack.BP_HatStack_C" (Math|Transform|MakeTransform "0, 0, 0" "0, 0, 0" "1,1,1") "Undefined" 0 0)))))))

(fn ConstructionScript)