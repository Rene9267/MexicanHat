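; BP_FinalHat is the end-of-game trigger that runs the ending when the player character overlaps it.
; It sets the character's EndGameDance flag and teleports it to the Sphere component's location.
; It then plays the LS_Ending level sequence with movement input disabled and the player visible, waits for the sequence's length, and opens the WinScene level.
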(event Collision|EventActorBeginOverlap
  (params (OtherActor :type Actor%20Object%20Reference))
  (bind _asthird_person_character (Utilities|Casting|CastToThirdPersonCharacter OtherActor))
  (Variables|/Game/ThirdPersonBP/Blueprints/ThirdPersonCharacter.ThirdPersonCharacter_C|SetEndGameDance _asthird_person_character true)
  (Transformation|Teleport _asthird_person_character (Transformation|GetWorldLocation (Variables|Default|GetSphere)) "0, 0, 0")
  (bind _outactor (Sequencer|Player|CreateLevelSequencePlayer "/Game/Animation/Cinematics/LS_Ending.LS_Ending" (Utilities|Struct|MakeMovieSceneSequencePlaybackSettings false (Utilities|Struct|MakeMovieSceneSequenceLoopCount 0) 1.0 0.0 false false true false false false true false)))
  (Sequencer|Player|Play (Variables|/Script/LevelSequence.LevelSequenceActor|GetSequencePlayer _outactor) :!class /Script/MovieScene.MovieSceneSequencePlayer)
  (Utilities|FlowControl|Delay (Class|TimeManagementBlueprintLibrary|ToSeconds(QualifiedFrameTime) (Class|MovieSceneSequencePlayer|GetEndTime (Variables|/Script/LevelSequence.LevelSequenceActor|GetSequencePlayer _outactor))))
  (Game|OpenLevel(byName) "WinScene"))

(fn ConstructionScript)