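; BP_Obstacle is an obstacle Blueprint built from a central Cube and four additional cube components.
; On BeginPlay, it shifts Cube1 to Cube4 outward along positive and negative world X and Y, and downward in Z, by the central Cube's bounds extents.
; The offsets adapt to the main Cube's size and add to each component's existing position, with an empty construction script.
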(event EventBeginPlay
  (bind _cube (Variables|Default|GetCube))
  (bind _boxextent (Collision|GetComponentBounds _cube))
  (bind _returnvalue (* (.z _boxextent) -1.0))
  (Class|SceneComponent|AddWorldTransform (Variables|Default|GetCube1) (Math|Transform|MakeTransform (Math|Vector|MakeVector (.x _boxextent) 0.0 _returnvalue) "0, 0, 0" "1,1,1") false false)
  (Class|SceneComponent|AddWorldTransform (Variables|Default|GetCube2) (Math|Transform|MakeTransform (Math|Vector|MakeVector (* (.x _boxextent) -1.0) 0.0 _returnvalue) "0, 0, 0" "1,1,1") false false)
  (Class|SceneComponent|AddWorldTransform (Variables|Default|GetCube3) (Math|Transform|MakeTransform (Math|Vector|MakeVector 0.0 (.y _boxextent) _returnvalue) "0, 0, 0" "1,1,1") false false)
  (Class|SceneComponent|AddWorldTransform (Variables|Default|GetCube4) (Math|Transform|MakeTransform (Math|Vector|MakeVector 0.0 (* (.y _boxextent) -1.0) _returnvalue) "0, 0, 0" "1,1,1") false false))

(fn ConstructionScript)